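; BP_Boid is a boid actor that acts as a contact hazard for the player's FlyingPawn.
; A startup delay after BeginPlay arms its damage flag, so early collisions are harmless.
; Once armed, a collision sphere overlap with a FlyingPawn damages shield and player, plays a quiet explosion sound and calls OnShot on itself.
; The graph holds no flocking or movement logic.
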(event `self.ReceiveBeginPlay`
  (`KismetSystemLibrary.Delay` 15.0)
  (set `self.CanDamagePlayer` true))

(event `self.CollisionSphere.OnComponentBeginOverlap`
  (params (OverlappedComponent :type "PrimitiveComponent Object Reference") (OtherActor :type "Actor Object Reference") (OtherComp :type "PrimitiveComponent Object Reference") (OtherBodyIndex :type Integer) (bFromSweep :type Boolean) (SweepResult :type "HitResult Structure (by ref)"))
  (bind _asflying_pawn (cast `/Game/Blueprints/FlyingPawn` OtherActor))
  (if (`self.CanDamagePlayer`)
    (`/Game/Blueprints/FlyingPawn.TakeDamageSheildPlayer` _asflying_pawn 50.0)
    (`/Game/Blueprints/FlyingPawn.TakeDamagePlayer` _asflying_pawn 5.0)
    (`GameplayStatics.PlaySoundAtLocation` "/Game/StarterContent/Audio/Explosion01.Explosion01" (`self.K2_GetActorLocation`) (struct) 0.1 1.0 0.0 null null null)
    (`self.OnShot` 100.0)))

(fn `UserConstructionScript`)