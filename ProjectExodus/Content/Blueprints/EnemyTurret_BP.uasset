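; Enemy turret that tracks and shoots the player's flying pawn and explodes when destroyed.
; PawnSensing snaps the actor toward a seen FlyingPawn and spawns EnemyProjectile_BP at the muzzle, throttled by a delay-reset flag.
; Player projectile overlaps on the capsule subtract health directly, with the death check subtracting the damage again.
; Separate clamped health and shield damage functions exist but are not called here.
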(event `self.PawnSensing.OnSeePawn`
  (params (Pawn :type "Pawn Object Reference"))
  ;[1 1 1] Turret rotation & shooting
  (bind _asflying_pawn (cast `/Game/Blueprints/FlyingPawn` Pawn))
  (`|ExecutionSequence`
    (:`then_0`
      (`self.K2_SetActorRotation` (`KismetMathLibrary.FindLookAtRotation` (`self.K2_GetActorLocation`) (`self.K2_GetActorLocation` _asflying_pawn))))
    (:`then_1`
      (if (`self.SpawnProjectile`)
        (`|SpawnActorFromClass` "/Game/Blueprints/EnemyProjectile_BP.EnemyProjectile_BP_C" (`SceneComponent.K2_GetComponentToWorld` (`self.ProjectileSpawnLoc`)) "AdjustIfPossibleButAlwaysSpawn" "OverrideRootScale" null null)
        (set `self.SpawnProjectile` false)
        (`KismetSystemLibrary.Delay` 0.5)
        (set `self.SpawnProjectile` true)))))

(event `self.CapsuleComponent.OnComponentBeginOverlap`
  (params (OverlappedComponent :type "PrimitiveComponent Object Reference") (OtherActor :type "Actor Object Reference") (OtherComp :type "PrimitiveComponent Object Reference") (OtherBodyIndex :type Integer) (bFromSweep :type Boolean) (SweepResult :type "HitResult Structure (by ref)"))
  (bind _returnvalue (- (`self.Health`) 5.0))
  (bind _asplayer_projectile_bp (cast `/Game/Blueprints/PlayerProjectile_BP` OtherActor))
  (`GameplayStatics.SpawnEmitterAtLocation` "/Game/StarterContent/Particles/P_Explosion.P_Explosion" SweepResult_ImpactPoint (struct) (100.0 100.0 100.0) false)
  (`self.K2_DestroyActor` _asplayer_projectile_bp)
  (set `self.Health` _returnvalue)
  (if (<= _returnvalue 0.0)
    (`GameplayStatics.SpawnEmitterAtLocation` "/Game/StarterContent/Particles/P_Explosion.P_Explosion" (`self.K2_GetActorLocation`) (struct) (100.0 100.0 100.0))
    (`self.K2_DestroyActor`)))

(fn `TakeDamageEnemy`
  (params (Damage :type "Float (double-precision)"))
  ;[1 1 1] Damage Function
  (bind _output_get (set `self.Health` (`KismetMathLibrary.FClamp` (- (`self.Health`) Damage) 0.0 100.0)))
  (set `self.HealthProgress` (/ _output_get 100.0)))

(fn `TakeDamageToShield`
  (params (ShieldDamage :type "Float (double-precision)"))
  ;[1 1 1] Damage Function
  (set `self.Shield` (`KismetMathLibrary.FClamp` (- (`self.Shield`) ShieldDamage) 0.0 50.0)))

(fn `UserConstructionScript`)