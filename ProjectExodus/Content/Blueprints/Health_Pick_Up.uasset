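; Health pickup actor that restores health to the FlyingPawn that touches it.
; On overlap with its collision component, it checks for the exact FlyingPawn class, adds a fixed amount to that pawn's Health, clamps it to the valid range and destroys itself.
; Tick is empty, and leftover disconnected nodes for an alternative health check and a yaw rotation never run.
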(event `self.ReceiveTick`
  (params (DeltaSeconds :type "Float (single-precision)")))

(event `self.Collison.OnComponentBeginOverlap`
  (params (OverlappedComponent :type "PrimitiveComponent Object Reference") (OtherActor :type "Actor Object Reference") (OtherComp :type "PrimitiveComponent Object Reference") (OtherBodyIndex :type Integer) (bFromSweep :type Boolean) (SweepResult :type "HitResult Structure (by ref)"))
  (if (== (`GameplayStatics.GetObjectClass` OtherActor) "/Game/Blueprints/FlyingPawn.FlyingPawn_C")
    (bind _asflying_pawn (cast `/Game/Blueprints/FlyingPawn` OtherActor))
    (set `/Game/Blueprints/FlyingPawn.Health` (`KismetMathLibrary.FClamp` (+ (`/Game/Blueprints/FlyingPawn.Health` _asflying_pawn) 25.0) 0.0 100.0) _asflying_pawn)
    (`self.K2_DestroyActor`)))

(fn `UserConstructionScript`)