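; Outpost is a destructible actor that loses health when player projectiles hit it.
; An overlap on its sphere collision accepts only PlayerProjectile_BP actors, destroys the projectile, spawns an explosion at the sweep impact point and removes one HP.
; When HP runs out, it spawns a much larger explosion at its own location and destroys itself.
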(event `self.SphereCollision.OnComponentBeginOverlap`
  (params (OverlappedComponent :type "PrimitiveComponent Object Reference") (OtherActor :type "Actor Object Reference") (OtherComp :type "PrimitiveComponent Object Reference") (OtherBodyIndex :type Integer) (bFromSweep :type Boolean) (SweepResult :type "HitResult Structure (by ref)"))
  (bind _asplayer_projectile_bp (cast `/Game/Blueprints/PlayerProjectile_BP` OtherActor))
  (`self.K2_DestroyActor` _asplayer_projectile_bp)
  (`GameplayStatics.SpawnEmitterAtLocation` "/Game/StarterContent/Particles/P_Explosion.P_Explosion" SweepResult_ImpactPoint (struct) (20.0 20.0 20.0))
  (bind _output_get (set `self.HP` (- (`self.HP`) 1)))
  (if (<= _output_get 0)
    (`GameplayStatics.SpawnEmitterAtLocation` "/Game/StarterContent/Particles/P_Explosion.P_Explosion" (`self.K2_GetActorLocation`) (struct) (500.0 500.0 500.0))
    (`self.K2_DestroyActor`)))

(fn `UserConstructionScript`)