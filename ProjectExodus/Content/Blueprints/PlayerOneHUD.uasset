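; PlayerOneHUD is a HUD Blueprint that draws a simple white square as a screen marker, apparently a crosshair.
; The DrawHUD event halves the viewport size and draws a small rectangle with its top-left corner at that point.
; An unconnected DrawTexture branch, noted as offsetting the crosshair vertically to align with the projectile, never runs and has no texture assigned.
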(event `self.ReceiveDrawHUD`
  (params (SizeX :type Integer) (SizeY :type Integer))
  (`self.DrawRect` (struct :`R` 1.0 :`G` 1.0 :`B` 1.0 :`A` 1.0) (`KismetMathLibrary.Conv_IntToDouble` (/ SizeX 2)) (`KismetMathLibrary.Conv_IntToDouble` (/ SizeY 2)) 10.0 10.0))

(event `DrawHud`)

(fn `UserConstructionScript`)