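; Player projectile that damages EnemyTurret_BP actors and removes itself after a short lifetime.
; Overlapping a turret's capsule always damages its shield; once the shield is depleted, the same hit also damages health, spawns an explosion and destroys the projectile.
; The projectile destroys the turret directly when its health runs out.
; Hits that leave the shield up do not destroy the projectile, which lives until its BeginPlay delay ends.
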(event `self.ProjectileMesh.OnComponentBeginOverlap`
  (params (OverlappedComponent :type "PrimitiveComponent Object Reference") (OtherActor :type "Actor Object Reference") (OtherComp :type "PrimitiveComponent Object Reference") (OtherBodyIndex :type Integer) (bFromSweep :type Boolean) (SweepResult :type "HitResult Structure (by ref)"))
  ;[1 1 1] DamageCalc - Jake
  (bind _asenemy_turret_bp (cast `/Game/Blueprints/EnemyTurret_BP` OtherActor))
  (if (== (`Character.CapsuleComponent` _asenemy_turret_bp) OtherComp)
    (`/Game/Blueprints/EnemyTurret_BP.TakeDamageToShield` _asenemy_turret_bp 10.0)
    (if (<= (`/Game/Blueprints/EnemyTurret_BP.Shield` _asenemy_turret_bp) 0.0)
      (`/Game/Blueprints/EnemyTurret_BP.TakeDamageEnemy` _asenemy_turret_bp 20.0)
      (`GameplayStatics.SpawnEmitterAtLocation` "/Game/StarterContent/Particles/P_Explosion.P_Explosion" (`self.K2_GetActorLocation`))
      (`self.K2_DestroyActor`)
      (if (<= (`/Game/Blueprints/EnemyTurret_BP.Health` _asenemy_turret_bp) 0.0)
        (`self.K2_DestroyActor` _asenemy_turret_bp)))))

(event `self.ReceiveBeginPlay`
  ;[1 1 1] DestroyActorAfterAmountOfTime - Jake
  (`KismetSystemLibrary.Delay` 0.5)
  (`self.K2_DestroyActor`))

(fn `UserConstructionScript`)