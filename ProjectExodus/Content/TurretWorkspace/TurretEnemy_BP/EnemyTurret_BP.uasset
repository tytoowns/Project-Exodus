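; Enemy turret that turns to face a sensed FlyingPawn and fires projectiles at it.
; PawnSensing drives both the instant look-at rotation and spawning Projectile_BP at the spawn point, throttled by a boolean gate and Delay cooldown.
; TakeDamageEnemy reduces clamped health and updates a normalized progress value, with no death handling.
; The health bar widget hookup is unfinished and, like a stray impulse snippet, never runs.
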(event `self.PawnSensing.OnSeePawn`
  (params (Pawn :type "Pawn Object Reference"))
  ;[1 1 1] Turret rotation & shooting
  (bind _asflying_pawn (cast `/Game/FlyingBP/Blueprints/FlyingPawn` Pawn))
  (`|ExecutionSequence`
    (:`then_0`
      (`self.K2_SetActorRotation` (`KismetMathLibrary.FindLookAtRotation` (`self.K2_GetActorLocation`) (`self.K2_GetActorLocation` _asflying_pawn))))
    (:`then_1`
      (if (`self.SpawnProjectile`)
        (`|SpawnActorFromClass` "/Game/TurretWorkspace/TurretEnemy_BP/EnemyProjectile_BP/Projectile_BP.Projectile_BP_C" (`SceneComponent.K2_GetComponentToWorld` (`self.ProjectileSpawnLoc`)) "AdjustIfPossibleButAlwaysSpawn" "OverrideRootScale" null null)
        (set `self.SpawnProjectile` false)
        (`KismetSystemLibrary.Delay` 1.5)
        (set `self.SpawnProjectile` true)))))

(event `self.ReceiveBeginPlay`
  ;[1 1 1] HealthBarWidget - WORK IN PROGRESS
)

(fn `TakeDamageEnemy`
  (params (Damage :type "Float (double-precision)"))
  (bind _output_get (set `self.Health` (`KismetMathLibrary.FClamp` (- (`self.Health`) Damage) 0.0 100.0)))
  (set `self.HealthProgress` (/ _output_get 100.0)))

(fn `UserConstructionScript`)