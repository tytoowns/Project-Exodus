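; Enemy turret projectile that damages the player's FlyingPawn and expires four seconds after spawning.
; On mesh overlap with the pawn's cockpit component, it damages the shield, then also damages health if the shield is depleted.
; Only that depleted-shield hit spawns an emitter and destroys the projectile.
; If health runs out, it destroys the pawn and opens LevelOne.
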(event `self.ProjectileMesh.OnComponentBeginOverlap`
  (params (OverlappedComponent :type "PrimitiveComponent Object Reference") (OtherActor :type "Actor Object Reference") (OtherComp :type "PrimitiveComponent Object Reference") (OtherBodyIndex :type Integer) (bFromSweep :type Boolean) (SweepResult :type "HitResult Structure (by ref)"))
  ;[1 1 1] DamageCalc - Jake
  (bind _asflying_pawn (cast `/Game/Blueprints/FlyingPawn` OtherActor))
  (if (== (`/Game/Blueprints/FlyingPawn.Cockpit_polySurface254` _asflying_pawn) OtherComp)
    (`/Game/Blueprints/FlyingPawn.TakeDamageSheildPlayer` _asflying_pawn 5.0)
    (if (<= (`/Game/Blueprints/FlyingPawn.Shield` _asflying_pawn) 0.0)
      (`/Game/Blueprints/FlyingPawn.TakeDamagePlayer` _asflying_pawn 10.0)
      (`GameplayStatics.SpawnEmitterAtLocation` null (`self.K2_GetActorLocation`))
      (`self.K2_DestroyActor`)
      (if (<= (`/Game/Blueprints/FlyingPawn.Health` _asflying_pawn) 0.0)
        (`self.K2_DestroyActor` _asflying_pawn)
        (`GameplayStatics.OpenLevel` "LevelOne")))))

(event `self.ReceiveBeginPlay`
  ;[1 1 1] DestroyActorAfterAmountOfTime - Jake
  (`KismetSystemLibrary.Delay` 4.0)
  (`self.K2_DestroyActor`))

(fn `UserConstructionScript`)