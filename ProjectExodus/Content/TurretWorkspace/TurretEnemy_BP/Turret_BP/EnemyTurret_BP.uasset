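; Enemy turret that detects the player's FlyingPawn through PawnSensing, turns to face it and shoots.
; On each sighting it snaps to a look-at rotation and spawns EnemyProjectile_BP at its spawn point, using a boolean and short Delay to limit fire rate.
; Separate functions apply clamped damage to Health (updating HealthProgress) and Shield.
; The destroy-on-zero-health check is disconnected, so the turret never destroys itself here.
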(event `self.PawnSensing.OnSeePawn`
  (params (Pawn :type "Pawn Object Reference"))
  ;[1 1 1] Turret rotation & shooting
  (bind _asflying_pawn (cast `/Game/Blueprints/FlyingPawn` Pawn))
  (`|ExecutionSequence`
    (:`then_0`
      (`self.K2_SetActorRotation` (`KismetMathLibrary.FindLookAtRotation` (`self.K2_GetActorLocation`) (`self.K2_GetActorLocation` _asflying_pawn))))
    (:`then_1`
      (if (`self.SpawnProjectile`)
        (`|SpawnActorFromClass` "/Game/TurretWorkspace/TurretEnemy_BP/Enemy_Projectile/EnemyProjectile_BP.EnemyProjectile_BP_C" (`SceneComponent.K2_GetComponentToWorld` (`self.ProjectileSpawnLoc`)) "AdjustIfPossibleButAlwaysSpawn" "OverrideRootScale" null null)
        (set `self.SpawnProjectile` false)
        (`KismetSystemLibrary.Delay` 0.2)
        (set `self.SpawnProjectile` true)))))

(fn `TakeDamageEnemy`
  (params (Damage :type "Float (double-precision)"))
  ;[1 1 1] Damage Function
  (bind _output_get (set `self.Health` (`KismetMathLibrary.FClamp` (- (`self.Health`) Damage) 0.0 100.0)))
  (set `self.HealthProgress` (/ _output_get 100.0)))

(fn `TakeDamageToShield`
  (params (ShieldDamage :type "Float (double-precision)"))
  ;[1 1 1] Damage Function
  (set `self.Shield` (`KismetMathLibrary.FClamp` (- (`self.Shield`) ShieldDamage) 0.0 50.0)))

(fn `UserConstructionScript`)